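; Player character for the LD_55 game, providing world-axis movement and a screenshot key through Enhanced Input.
; On BeginPlay it adds the IMC_LD55 mapping context to the controlling PlayerController.
; The North and East move actions feed world X and Y input straight into CharacterMovement, independent of camera or actor rotation.
; The screenshot action triggers a gameplay automation screenshot when it starts.
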(event `self.ReceiveBeginPlay`
  (bind _asplayer_controller (cast `PlayerController` (`self.GetController`)))
  (message `EnhancedInputSubsystemInterface.AddMappingContext` (pcsubsystem `EnhancedInputLocalPlayerSubsystem` _asplayer_controller) "/Game/LD_55_Custom/Blueprints/Controls/IMC_LD55.IMC_LD55" 0 (make `ModifyContextOptions` true)))

(event `EnhancedInput|/Game/LD_55_Custom/Blueprints/Controls/IA_Move_East`
  (params (ActionValue :type "Float (double-precision)") (ElapsedSeconds :type "Float (double-precision)") (TriggeredSeconds :type "Float (double-precision)") (InputAction :type "InputAction Object Reference" :default "/Game/LD_55_Custom/Blueprints/Controls/IA_Move_East.IA_Move_East"))
  (:`Triggered`
    (`PawnMovementComponent.AddInputVector` (`self.CharacterMovement`) (`KismetMathLibrary.MakeVector` 0.0 ActionValue) false)))

(event `EnhancedInput|/Game/LD_55_Custom/Blueprints/Controls/IA_Move_North`
  (params (ActionValue :type "Float (double-precision)") (ElapsedSeconds :type "Float (double-precision)") (TriggeredSeconds :type "Float (double-precision)") (InputAction :type "InputAction Object Reference" :default "/Game/LD_55_Custom/Blueprints/Controls/IA_Move_North.IA_Move_North"))
  (:`Triggered`
    (`PawnMovementComponent.AddInputVector` (`self.CharacterMovement`) (`KismetMathLibrary.MakeVector` ActionValue) false)))

(event `EnhancedInput|/Game/LD_55_Custom/Blueprints/Controls/IA_ScreenShot`
  (params (ActionValue :type Boolean) (ElapsedSeconds :type "Float (double-precision)") (TriggeredSeconds :type "Float (double-precision)") (InputAction :type "InputAction Object Reference" :default "/Game/LD_55_Custom/Blueprints/Controls/IA_ScreenShot.IA_ScreenShot"))
  (:`Started`
    (`AutomationUtilsBlueprintLibrary.TakeGameplayAutomationScreenshot` "")))

(fn `UserConstructionScript`)