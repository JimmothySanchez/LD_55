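; BP_NPC_Base is a base Blueprint for NPCs that displays a widget when the player is nearby and the NPC has something to say, as flagged by HasTalk.
; Every Tick it polls whether its Sphere component overlaps the player's controlled pawn, then sets the Widget component's user widget visible or hidden.
; BeginPlay and the construction script are empty, and it contains no dialogue logic.
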(event `self.ReceiveBeginPlay`)

(event `self.ReceiveTick`
  (params (DeltaSeconds :type "Float (single-precision)"))
  (if (and (`PrimitiveComponent.IsOverlappingActor` (`self.Sphere`) (`Controller.K2_GetPawn` (`GameplayStatics.GetPlayerController` 0))) (`self.HasTalk`))
    (`Widget.SetVisibility` (`WidgetComponent.GetWidget` (`self.Widget`)) "Visible")
    (else
      (`Widget.SetVisibility` (`WidgetComponent.GetWidget` (`self.Widget`)) "Hidden"))))

(fn `UserConstructionScript`)