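; BP_ProfOak is the Professor Oak NPC, which starts its own dialog when its talk button fires.
; On BeginPlay it binds to the talk-start event of the WDG_TalkButton held by its Widget component.
; That event creates a WDG_DLG_POK_01 dialog widget and hands it to the GM_LD_55 game mode through CallDialogStarted.
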(event `self.ReceiveBeginPlay`
  (bind _aswdg_talk_button (cast `/Game/LD_55_Custom/Blueprints/UI/WDG_TalkButton` (`WidgetComponent.GetWidget` (`self.Widget`))))
  (add `/Game/LD_55_Custom/Blueprints/UI/WDG_TalkButton.TalkStart` _aswdg_talk_button (delegate `CustomEvent_0`))
  (`parent.ReceiveBeginPlay`))

(event `CustomEvent_0`
  (bind _asgm_ld_55 (cast `/Game/LD_55_Custom/Blueprints/Logic/GM_LD_55` (`GameplayStatics.GetGameMode`)))
  (bind _returnvalue (`|CreateWidget` "/Game/LD_55_Custom/Blueprints/UI/Dialogs/WDG_DLG_POK_01.WDG_DLG_POK_01_C"))
  (`/Game/LD_55_Custom/Blueprints/Logic/GM_LD_55.DialogStarted` _asgm_ld_55 _returnvalue))

(fn `UserConstructionScript`
  (`parent.UserConstructionScript`))