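; Player controller that switches the player's input and HUD between overworld and combat modes.
; On BeginPlay it creates both HUD widgets, enables Game and UI input with a visible cursor, and starts in overworld mode.
; It binds to the GM_LD_55 game mode's combat started and ended events, each swapping Enhanced Input mapping contexts and on-screen HUD widgets.
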(event `self.ReceiveBeginPlay`
  (`|ExecutionSequence`
    (:`then_0`
      (bind _returnvalue (`|CreateWidget` "/Game/LD_55_Custom/Blueprints/UI/WDG_HUD_Overworld.WDG_HUD_Overworld_C"))
      (set `self.OverworldHud` _returnvalue)
      (bind _returnvalue_2 (`|CreateWidget` "/Game/LD_55_Custom/Blueprints/UI/WDG_HUD_Combat.WDG_HUD_Combat_C"))
      (set `self.CombatHud` _returnvalue_2))
    (:`then_1`
      ;[1 1 1] Comment
      (`WidgetBlueprintLibrary.SetInputMode_GameAndUIEx` self null "DoNotLock" false)
      (set `self.bShowMouseCursor` true)
      (`self.SetOverworldContext`))
    (:`then_2`
      ;[1 1 1] InitCombat
      (bind _asgm_ld_55 (cast `/Game/LD_55_Custom/Blueprints/Logic/GM_LD_55` (`GameplayStatics.GetGameMode`)))
      (add `/Game/LD_55_Custom/Blueprints/Logic/GM_LD_55.CombatEventStarted` _asgm_ld_55 (delegate `CustomEvent`)))
    (:`then_3`
      (bind _asgm_ld_55_2 (cast `/Game/LD_55_Custom/Blueprints/Logic/GM_LD_55` (`GameplayStatics.GetGameMode`)))
      (add `/Game/LD_55_Custom/Blueprints/Logic/GM_LD_55.CombatEnded` _asgm_ld_55_2 (delegate `CustomEvent_0`)))))

(event `CustomEvent`
  ;[1 1 1] InitCombat
  (`self.SetCombatContext`))

(event `CustomEvent_0`
  ;[1 1 1] InitCombat
  (`self.SetOverworldContext`))

(fn `SetCombatContext`
  (bind _returnvalue (pcsubsystem `EnhancedInputLocalPlayerSubsystem` self))
  (`EnhancedInputSubsystemInterface.RemoveMappingContext` _returnvalue "/Game/LD_55_Custom/Blueprints/Controls/IMC_LD55_Overworld.IMC_LD55_Overworld" (struct))
  (`EnhancedInputSubsystemInterface.AddMappingContext` _returnvalue "/Game/LD_55_Custom/Blueprints/Controls/IMC_LD55_Combat.IMC_LD55_Combat" 0 (struct))
  (`Widget.RemoveFromParent` (`self.OverworldHud`))
  (`UserWidget.AddToPlayerScreen` (`self.CombatHud`) 0))

(fn `SetOverworldContext`
  (bind _returnvalue (pcsubsystem `EnhancedInputLocalPlayerSubsystem` self))
  (`EnhancedInputSubsystemInterface.RemoveMappingContext` _returnvalue "/Game/LD_55_Custom/Blueprints/Controls/IMC_LD55_Combat.IMC_LD55_Combat" (struct))
  (`EnhancedInputSubsystemInterface.AddMappingContext` _returnvalue "/Game/LD_55_Custom/Blueprints/Controls/IMC_LD55_Overworld.IMC_LD55_Overworld" 0 (struct))
  (`Widget.RemoveFromParent` (`self.CombatHud`))
  (`UserWidget.AddToPlayerScreen` (`self.OverworldHud`) 0))

(fn `UserConstructionScript`)