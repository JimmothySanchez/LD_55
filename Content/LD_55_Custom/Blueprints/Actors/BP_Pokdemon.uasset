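; BP_Pokdemon is the actor for a Pokdemon creature on the Player or AI team, with its mesh and stats held in PokdemonInfo.
; On BeginPlay it applies the body mesh from that info.
; Its SceneCaptureComponent2D shows only itself and renders to the player or enemy render target according to Team.
; Refresh restores Health and Power to their maximums.
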(event `self.ReceiveBeginPlay`
  (`KismetArrayLibrary.Array_Add` (`SceneCaptureComponent.ShowOnlyActors` (`self.SceneCaptureComponent2D`)) self)
  (`self.InitFromInfo`)
  (switch `/Game/LD_55_Custom/Blueprints/Logic/Data/Pokdemons/Enum_Teams` (`self.Team`)
    (:`NewEnumerator0`
      (set `SceneCaptureComponent2D.TextureTarget` "/Game/LD_55_Custom/Blueprints/UI/RT_PlayerPokdemon.RT_PlayerPokdemon" (`self.SceneCaptureComponent2D`)))
    (:`NewEnumerator1`
      (set `SceneCaptureComponent2D.TextureTarget` "/Game/LD_55_Custom/Blueprints/UI/RT_EnemyPokdemon.RT_EnemyPokdemon" (`self.SceneCaptureComponent2D`)))))

(fn `InitFromInfo`
  (`StaticMeshComponent.SetStaticMesh` (`self.BodyMesh`) (`.Mesh_5_B076EA3F48D3162DE99C249DAFDBE0FB` (break `/Game/LD_55_Custom/Blueprints/Logic/Data/Pokdemons/ST_Pokdemon_Info` (`/Game/LD_55_Custom/Blueprints/Logic/Data/Pokdemons/BP_Pokdemon_Base.Info` (`self.PokdemonInfo`))))))

(fn `Refresh`
  (bind (_name _type _mesh _maxhealth _maxpower) (break `/Game/LD_55_Custom/Blueprints/Logic/Data/Pokdemons/ST_Pokdemon_Info` (`/Game/LD_55_Custom/Blueprints/Logic/Data/Pokdemons/BP_Pokdemon_Base.Info` (`self.PokdemonInfo`))))
  (setmembers `/Game/LD_55_Custom/Blueprints/Logic/Data/Pokdemons/ST_Pokdemon_Info` :`StructRef` (`/Game/LD_55_Custom/Blueprints/Logic/Data/Pokdemons/BP_Pokdemon_Base.Info` (`self.PokdemonInfo`)) :`Health` _maxhealth :`Power` _maxpower))

(fn `UserConstructionScript`)