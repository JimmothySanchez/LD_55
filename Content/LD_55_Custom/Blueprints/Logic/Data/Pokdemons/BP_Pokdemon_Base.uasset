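; BP_Pokdemon_Base is the base data Blueprint for a Pokdemon creature, holding its stats, actions and leveling logic.
; Init packs the configured defaults into an STPokdemonInfo struct, which later functions modify.
; CheckLevelUp compares Experience to a threshold that doubles each level; leveling clears experience, raises max health, power and strength, then refills health and power.
; A helper scales the reward by level.
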(fn `CheckLevelUp`
  (if (>= (`self.Experience`) (`self.GetNextLevelExp`))
    (`self.LevelUp`)))

(fn `GetNextLevelExp`
  (returns (ReturnValue :type Integer))
  (return (`KismetMathLibrary.FFloor` (`KismetMathLibrary.MultiplyMultiply_FloatFloat` 2.0 (`KismetMathLibrary.Conv_IntToDouble` (+ (`self.Level`) 3))))))

(fn `GetRewardCalc`
  (returns (Reward :type Integer))
  (return (* (`self.Reward`) (`self.Level`))))

(fn `Init`
  (set `self.Info` (make `/Game/LD_55_Custom/Blueprints/Logic/Data/Pokdemons/ST_Pokdemon_Info` (`self.Name`) (`self.Type`) null (`self.Initail Max Health`) (`self.Initial Max Power`) (`self.InitialStrength`) (`self.Reward`) (`self.InitialHealth`) (`self.InitialPower`) (`self.Level`) false 0 (`self.Icon`) (`self.Actions`))))

(fn `LevelUp`
  (bind (_name _type _mesh _maxhealth _maxpower _strength) (break `/Game/LD_55_Custom/Blueprints/Logic/Data/Pokdemons/ST_Pokdemon_Info` (`self.Info`)))
  (`/Engine/EditorBlueprintResources/StandardMacros.IncrementInt` (`self.Level`)
    (:`  `
      (set `self.Experience` 0)
      (setmembers `/Game/LD_55_Custom/Blueprints/Logic/Data/Pokdemons/ST_Pokdemon_Info` :`StructRef` (`self.Info`) :`MaxHealth` (+ _maxhealth 1) :`MaxPower` (+ _maxpower 2) :`Strength` (+ _strength 1))
      (`self.ResetHealthAndPower`))))

(fn `ResetHealthAndPower`
  (bind (_name _type _mesh _maxhealth _maxpower) (break `/Game/LD_55_Custom/Blueprints/Logic/Data/Pokdemons/ST_Pokdemon_Info` (`self.Info`)))
  (setmembers `/Game/LD_55_Custom/Blueprints/Logic/Data/Pokdemons/ST_Pokdemon_Info` :`StructRef` (`self.Info`) :`Health` _maxhealth :`Power` _maxpower))