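; Game mode for the LD55 game that tracks combat and dialog state in response to bound events.
; Dialog start shows the supplied widget and removes the overworld Enhanced Input mapping context, which dialog end restores; combat handlers only toggle InCombat.
; HandleRandomItemEvent grants an Ouija or Vinyl item to the game instance inventory, shows an alert and removes overworld input, but its bound event handler is empty.
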(event `CustomEvent`
  ;[1 1 1] Combat Events
  (`self.HandleCombatStart`))

(event `CustomEvent_0`
  ;[1 1 1] Combat Events
  (`self.HandleCombatEnd`))

(event `self.ReceiveBeginPlay`
  (`|ExecutionSequence`
    (:`then_0`
      ;[1 1 1] Combat Events
      (add `self.CombatEventStarted` (delegate `CustomEvent`))
      (add `self.CombatEnded` (delegate `CustomEvent_0`)))
    (:`then_1`
      (add `self.DialogStarted` (delegate `CustomEvent_3`))
      (add `self.DialogEnded` (delegate `CustomEvent_4`)))
    (:`then_2`
      (add `self.RandomItemEvent` (delegate `CustomEvent_6`)))))

(event `CustomEvent_3` :!signature `self.DialogStarted`
  (params (DialogEntryWidget :type "UserWidget Object Reference"))
  (`self.StartDialog` DialogEntryWidget))

(event `CustomEvent_4`
  (set `self.InDialog` false)
  (`self.HandleDialogEnd`))

(event `CustomEvent_6`)

(fn `HandleCombatEnd`
  (set `self.InCombat` false))

(fn `HandleCombatStart`
  (set `self.InCombat` true))

(fn `HandleDialogEnd`
  (`EnhancedInputSubsystemInterface.AddMappingContext` (pcsubsystem `EnhancedInputLocalPlayerSubsystem` (`GameplayStatics.GetPlayerController` 0)) "/Game/LD_55_Custom/Blueprints/Controls/IMC_LD55_Overworld.IMC_LD55_Overworld" 0 (struct)))

(fn `HandleRandomItemEvent`
  (locals (ItemType :type "/Game/LD_55_Custom/Blueprints/Logic/Data/Inventory/BP_InventoryItem_Base Class Reference"))
  (`|ExecutionSequence`
    (:`then_0`
      (switch `int` (`KismetMathLibrary.RandomInteger` 2)
        (:`0`
          (set `local.ItemType` "/Game/LD_55_Custom/Blueprints/Logic/Data/Inventory/BP_Item_Ouija.BP_Item_Ouija_C"))
        (:`1`
          (set `local.ItemType` "/Game/LD_55_Custom/Blueprints/Logic/Data/Inventory/BP_Item_Vinyl.BP_Item_Vinyl_C"))))
    (:`then_1`
      (bind _returnvalue (`|GenericCreateObject` (`local.ItemType`)))
      (bind _asbp_inventory_item_base (cast `/Game/LD_55_Custom/Blueprints/Logic/Data/Inventory/BP_InventoryItem_Base` _returnvalue))
      (bind _asgi_ld55 (cast `/Game/LD_55_Custom/Blueprints/Logic/GI_LD55` (`GameplayStatics.GetGameInstance`)))
      (`KismetArrayLibrary.Array_Add` (`/Game/LD_55_Custom/Blueprints/Logic/GI_LD55.ItemInventory` _asgi_ld55) _asbp_inventory_item_base)
      (bind _returnvalue_2 (`|CreateWidget` "/Game/LD_55_Custom/Blueprints/UI/WDG_NewItemAlert.WDG_NewItemAlert_C" null _asbp_inventory_item_base))
      (`UserWidget.AddToPlayerScreen` _returnvalue_2 0)
      (`EnhancedInputSubsystemInterface.RemoveMappingContext` (pcsubsystem `EnhancedInputLocalPlayerSubsystem` (`GameplayStatics.GetPlayerController` 0)) "/Game/LD_55_Custom/Blueprints/Controls/IMC_LD55_Overworld.IMC_LD55_Overworld" (struct)))))

(fn `StartDialog`
  (params (DialogEntryWidget :type "UserWidget Object Reference"))
  (set `self.InDialog` true)
  (`EnhancedInputSubsystemInterface.RemoveMappingContext` (pcsubsystem `EnhancedInputLocalPlayerSubsystem` (`GameplayStatics.GetPlayerController` 0)) "/Game/LD_55_Custom/Blueprints/Controls/IMC_LD55_Overworld.IMC_LD55_Overworld" (struct))
  (`UserWidget.AddToPlayerScreen` DialogEntryWidget 0))

(fn `UserConstructionScript`)