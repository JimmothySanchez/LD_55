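; BP_Road is a spline-driven road actor that builds its mesh in the Construction Script, with no active runtime logic.
; It walks the spline in fixed-length steps, including a final step for the remainder, and adds a spline mesh component using MeshType for each.
; Each piece deforms along X, taking start and end positions and tangents from the spline by distance in local space.
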(fn `UserConstructionScript`
  (locals (lclSplineMesh :type "SplineMeshComponent Object Reference") (lclRoadLength :type "Float (double-precision)" :default 0.0) (lclCurrentPointIndex :type Integer))
  (bind _returnvalue (* (`local.lclRoadLength`) (`local.lclCurrentPointIndex`)))
  (bind _returnvalue_2 (* (`local.lclRoadLength`) (+ (`local.lclCurrentPointIndex`) 1)))
  (bind _output_get (set `local.lclRoadLength` 1500.0))
  (for _index (range (+ (`KismetMathLibrary.FFloor` (/ (`SplineComponent.GetSplineLength` (`self.Spline`)) _output_get)) 1))
    (set `local.lclCurrentPointIndex` _index)
    (bind _returnvalue_3 (`AddComponent|NODE_AddSplineMeshComponent-0`))
    (bind _output_get_2 (set `local.lclSplineMesh` _returnvalue_3))
    (`SplineMeshComponent.SetForwardAxis` _output_get_2 "X" true)
    (`StaticMeshComponent.SetStaticMesh` (`local.lclSplineMesh`) (`self.MeshType`))
    (`|ExecutionSequence`
      (:`then_0`
        ;[1 1 1] Start
        (`SplineMeshComponent.SetStartAndEnd` (`local.lclSplineMesh`) (`SplineComponent.GetLocationAtDistanceAlongSpline` (`self.Spline`) _returnvalue "Local") (`SplineComponent.GetTangentAtDistanceAlongSpline` (`self.Spline`) _returnvalue "Local") (`SplineComponent.GetLocationAtDistanceAlongSpline` (`self.Spline`) _returnvalue_2 "Local") (`SplineComponent.GetTangentAtDistanceAlongSpline` (`self.Spline`) _returnvalue_2 "Local") true)))))